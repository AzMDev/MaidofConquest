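; Enemy AI character that roams randomly, chases the player on sight and plays a melee attack montage.
; Tick drives delayed roaming; PawnSensing starts the chase at a randomized speed, with a sighting flag that clears after a short delay.
; Reaching the player triggers the attack behind a cooldown flag.
; Damage lowers health, pausing movement for random hit reactions, or at zero playing a random death, disabling collision and later destroying the actor.
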(event OnSeePawn(PawnSensing)
  (params (Pawn :type Pawn%20Object%20Reference))
  (Utilities|Casting|CastToUe4ASP_Character Pawn)
  (Utilities|FlowControl|Sequence
    (:then_0
      (Variables|Default|SetisSeeingPlayer true)
      (CallFunction|FollowPlayer)
      (Variables|/Script/Engine.CharacterMovementComponent|SetMaxWalkSpeed (Variables|Character|GetCharacterMovement) (Utilities|Select :Index (Math|Random|RandomInteger 4) :Option%200 4e+02 :Option%201 4.5e+02 :Option%202 5e+02 :Option%203 5.5e+02 :Option%204 6e+02)))
    (:then_1
      (Utilities|FlowControl|Delay 0.5)
      (Variables|Default|SetisSeeingPlayer false))))

(event Custom|FollowPlayer
  (if (not (Variables|Default|GetisDead))
    (Variables|Default|SetcanAttack true)
    (if (Variables|Default|GetisSeeingPlayer)
      (AI|AIMoveTo self "0, 0, 0" (Game|GetPlayerCharacter 0) 1e+02 false
        (:OnSuccess
          (if (Variables|Default|GetcanAttack)
            (Variables|Default|SetcanAttack false)
            (if (not (Variables|Default|GetisDead))
              (Animation|PlayAnimMontage "/Game/MaidOfConquest_Content/Animations/Attack/Paired_CounterPunch_PalmStrike_Att_UE5_Montage.Paired_CounterPunch_PalmStrike_Att_UE5_Montage" 1.0 "None")
              (Utilities|FlowControl|Delay 1.0)
              (Variables|Default|SetcanAttack true))))))))

(event EventTick
  (params (DeltaSeconds :type Float%20%28single-precision%29))
  ;[1 1 1] AI Random Roam
  (if (and (not (Variables|Default|GetisSeeingPlayer)) (not (Variables|Default|GetisMoving)))
    (Utilities|FlowControl|Delay (Math|Random|RandomFloatinRange 2.0 5.0))
    (Variables|Default|SetisMoving true)
    (AI|AIMoveTo self (.RandomLocation (AI|Navigation|GetRandomReachablePointinRadius (Transformation|GetActorLocation) 1e+03 0 0)) 0 5.0 false
      (:OnSuccess
        _)
      (:OnFail
        _))
    (Variables|Default|SetisMoving false)))

(event Game|Damage|EventAnyDamage
  (params (Damage :type Float%20%28single-precision%29) (DamageType :type Damage%20Type%20Object%20Reference) (InstigatedBy :type Controller%20Object%20Reference) (DamageCauser :type Actor%20Object%20Reference))
  (bind _returnvalue (Transformation|GetActorLocation))
  (if (not (Variables|Default|GetisDead))
    (bind _output_get (Variables|Default|SetHealth (Math|Float|Clamp(Float) (- (Variables|Default|GetHealth) Damage) 0.0 1e+02)))
    (if (== _output_get 0.0)
      (Audio|PlaySoundatLocation "/Game/MaidOfConquest_Content/SFX/Death/DeathCue.DeathCue" _returnvalue "0, 0, 0" 1.0 1.0 0.0 0 0 0 0)
      (Pawn|Components|CharacterMovement|DisableMovement (Variables|Character|GetCharacterMovement))
      (Variables|Default|SetisDead true)
      (Animation|PlayAnimMontage (Utilities|Select :Index (Math|Random|RandomInteger 2) :Option%200 "/Game/MaidOfConquest_Content/Animations/Death_Anim/Death_2_Montage.Death_2_Montage" :Option%201 "/Game/MaidOfConquest_Content/Animations/Death_Anim/Death_3_Montage.Death_3_Montage" :Option%202 "/Game/MaidOfConquest_Content/Animations/Death_Anim/Death_4_Montage.Death_4_Montage") 1.0 "None")
      (Collision|SetCollisionEnabled (Variables|Collision|GetCapsuleComponent) "NoCollision")
      (Utilities|FlowControl|Delay 6e+01)
      (Actor|DestroyActor)
      (else
        (Audio|PlaySoundatLocation "/Game/MaidOfConquest_Content/SFX/Damage_Male/DamageCue.DamageCue" _returnvalue "0, 0, 0" 1.0 1.0 0.0 0 0 0 0)
        (Pawn|Components|CharacterMovement|DisableMovement (Variables|Character|GetCharacterMovement))
        (bind _returnvalue_2 (Animation|PlayAnimMontage (Utilities|Select :Index (Math|Random|RandomInteger 3) :Option%200 "/Game/MaidOfConquest_Content/Animations/Hit_Anim/Hit_1_Montage.Hit_1_Montage" :Option%201 "/Game/MaidOfConquest_Content/Animations/Hit_Anim/Hit_2_Montage.Hit_2_Montage" :Option%202 "/Game/MaidOfConquest_Content/Animations/Hit_Anim/Hit_3_Montage.Hit_3_Montage" :Option%203 "/Game/MaidOfConquest_Content/Animations/Hit_Anim/Hit_4_Montage.Hit_4_Montage") 1.0 "None"))
        (Utilities|FlowControl|Delay _returnvalue_2)
        (if (not (Variables|Default|GetisDead))
          (Pawn|Components|CharacterMovement|SetMovementMode (Variables|Character|GetCharacterMovement) "MOVE_Walking" 0))))))

(fn ConstructionScript)