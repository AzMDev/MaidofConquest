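; Enemy AI character that chases the player on sight and plays a melee attack montage when it reaches them.
; PawnSensing sets a seen flag and triggers FollowPlayer, which uses AI MoveTo and gates the montage with a one-second cooldown.
; Tick halts movement until the first sighting; the seen flag is never cleared, and each FollowPlayer call re-enables attacking.
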(event OnSeePawn(PawnSensing)
  (params (Pawn :type Pawn%20Object%20Reference))
  (Variables|Default|SetisSeeingPlayer true)
  (CallFunction|FollowPlayer))

(event Custom|FollowPlayer
  (Variables|Default|SetcanAttack true)
  (if (Variables|Default|GetisSeeingPlayer)
    (AI|AIMoveTo self "0, 0, 0" (Game|GetPlayerCharacter 0) 7e+01 false
      (:OnSuccess
        (if (Variables|Default|GetcanAttack)
          (Variables|Default|SetcanAttack false)
          (Animation|PlayAnimMontage "/Game/MaidOfConquest/Animations/Paired_CounterPunch_PalmStrike_Att_UE5_Montage.Paired_CounterPunch_PalmStrike_Att_UE5_Montage" 1.0 "None")
          (Utilities|FlowControl|Delay 1.0)
          (Variables|Default|SetcanAttack true))))))

(event EventBeginPlay)

(event Collision|EventActorBeginOverlap
  (params (OtherActor :type Actor%20Object%20Reference)))

(event EventTick
  (params (DeltaSeconds :type Float%20%28single-precision%29))
  (if (not (Variables|Default|GetisSeeingPlayer))
    (Components|Movement|StopMovementImmediately (Variables|Character|GetCharacterMovement))))

(fn ConstructionScript)